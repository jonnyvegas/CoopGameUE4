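; Prototype grenade for the grenade launcher that explodes one second after it spawns.
; Explode spawns an explosion particle effect, applies full radial damage within its Sphere component's radius, ignoring itself, then destroys the actor.
; A trailing loop casts overlapping actors to BP_TargetDummy but does nothing further, as the radial impulse and debug sphere nodes are disconnected.
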(event Custom|Explode!
  (bind _returnvalue (Transformation|GetActorLocation))
  (Effects|SpawnEmitteratLocation "/Game/WeaponEffects/Explosion/P_Explosion.P_Explosion" _returnvalue)
  (Game|Damage|ApplyRadialDamage 1e+02 _returnvalue (Variables|/Script/Engine.SphereComponent|GetSphereRadius (Variables|Default|GetSphere)) "/Script/Engine.DamageType" (Utilities|Array|MakeArray self) self 0 true "ECC_Visibility")
  (Actor|DestroyActor)
  (for _array_element (Collision|GetOverlappingActors (Variables|Default|GetSphere) 0 :!class /Script/Engine.PrimitiveComponent)
    (bind _asbp_target_dummy (Utilities|Casting|CastToBP_TargetDummy _array_element))))

(event EventBeginPlay
  (Utilities|FlowControl|Delay 1.0)
  (CallFunction|Explode!))

(event Collision|EventActorBeginOverlap
  (params (OtherActor :type Actor%20Object%20Reference)))

(event EventTick
  (params (DeltaSeconds :type Float%20%28single-precision%29)))

(fn ConstructionScript)